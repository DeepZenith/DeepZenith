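; MainPlantBP is the central plant prop, which reacts and can die, with sound feedback for each.
; React plays a happy cue at the plant's location and calls the React dispatcher.
; Muerte plays a sad cue, advances the MissionFinal mission's progress by one, and calls the Death dispatcher.
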(event Custom|Muerte
  (Audio|PlaySoundatLocation "/Game/SonidosFX/Planto/planta_sad_Cue.planta_sad_Cue" (Transformation|GetWorldLocation (Variables|Default|GetMainPlant)))
  (Default|UpdateProgress (Variables|Default|GetMissionFinal) 1)
  (Default|CallDeathDispatcher))

(event Custom|React
  (Audio|PlaySoundatLocation "/Game/SonidosFX/Planto/planta_happy_Cue.planta_happy_Cue" (Transformation|GetWorldLocation (Variables|Default|GetMainPlant)))
  (Default|CallReactDispatcher))

(fn ConstructionScript)