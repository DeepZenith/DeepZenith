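; CajaAbono is a prop with two doors that respond to a key-gated trigger.
; When KeyTrigger is overlapped with KeyPicked set, a FirstPersonCharacter check and DoOnce play a timeline that swings the doors in opposite directions.
; Without the key, any overlapping actor restarts a second timeline that moves them by a smaller factor.
; Both timelines add their scaled track value as relative yaw each update, rather than setting absolute angles.
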(event OnComponentBeginOverlap(keyTrigger)
  (params (OverlappedComponent :type Primitive%20Component%20Object%20Reference) (OtherActor :type Actor%20Object%20Reference) (OtherComp :type Primitive%20Component%20Object%20Reference) (OtherBodyIndex :type Integer) (bFromSweep :type Boolean) (SweepResult :type Hit%20Result%20Structure%20%28by%20ref%29))
  (if (Variables|Default|GetkeyPicked)
    (Utilities|Casting|CastToFirstPersonCharacter OtherActor)
    (Utilities|FlowControl|DoOnce false
      (:Completed
        (bind _newtrack_0 (Timeline|Timeline_1 Play)
          (:Update
            (Transformation|AddLocalRotation (Variables|Default|Getpuertaizq) (Math|Rotator|MakeRotator 0.0 0.0 (* _newtrack_0 2.5)) false false)
            (Transformation|AddLocalRotation (Variables|Default|Getpuertader) (Math|Rotator|MakeRotator 0.0 0.0 (* -1 (* _newtrack_0 2.5))) false false)))))
    (else
      (bind _newtrack_0_2 (Timeline|Timeline_0 PlayFromStart)
        (:Update
          (Transformation|AddLocalRotation (Variables|Default|Getpuertaizq) (Math|Rotator|MakeRotator 0.0 0.0 (/ _newtrack_0_2 3.0)) false false)
          (Transformation|AddLocalRotation (Variables|Default|Getpuertader) (Math|Rotator|MakeRotator 0.0 0.0 (* -1 (/ _newtrack_0_2 3.0))) false false))))))

(event EventBeginPlay)

(event Collision|EventActorBeginOverlap
  (params (OtherActor :type Actor%20Object%20Reference)))

(event EventTick
  (params (DeltaSeconds :type Float%20%28single-precision%29)))

(fn ConstructionScript)