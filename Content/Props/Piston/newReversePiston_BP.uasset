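; Piston prop that starts cycling on BeginPlay, sliding its box component down and back up along Z.
; Two eased MoveComponentTo calls chain through their completion callbacks, each followed by a short pause.
; STOPP sets a flag checked after each pause, so the current stroke finishes before halting.
; RESUMM clears it and uses the Ida direction flag to restart the appropriate stroke.
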(event Custom|STOPP
  (Variables|Default|Setstop true))

(event Custom|RESUMM
  (bind _piston_low_box008 (Variables|Default|GetPiston_Low_Box008))
  (Variables|Default|Setstop false)
  (if (Variables|Default|GetIda)
    (Components|MoveComponentTo _piston_low_box008 "0, 0,50.000000" "0, 0, 0" false true 3.0 false :!label _label)
    (Variables|Default|SetIda false)
    (Utilities|FlowControl|Delay 1.0)
    (if (not (Variables|Default|Getstop))
      (Components|MoveComponentTo _piston_low_box008 "0, 0,-500.000000" "0, 0, 0" false true 3.0 false :!label _label_2)
      (Variables|Default|SetIda true)
      (Utilities|FlowControl|Delay 1.0)
      (if (not (Variables|Default|Getstop))
        (goto _label)))
    (else
      (goto _label_2))))

(event EventBeginPlay
  (bind _piston_low_box008 (Variables|Default|GetPiston_Low_Box008))
  (Variables|Default|SetIda false)
  (Components|MoveComponentTo _piston_low_box008 "0, 0,-500.000000" "0, 0, 0" false true 3.0 false :!label _label)
  (Variables|Default|SetIda true)
  (Utilities|FlowControl|Delay 1.0)
  (if (not (Variables|Default|Getstop))
    (Components|MoveComponentTo _piston_low_box008 "0, 0,50.000000" "0, 0, 0" false true 3.0 false)
    (Variables|Default|SetIda false)
    (Utilities|FlowControl|Delay 1.0)
    (if (not (Variables|Default|Getstop))
      (goto _label))))

(fn ConstructionScript)