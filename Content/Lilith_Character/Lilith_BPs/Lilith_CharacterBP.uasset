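; Lilith character Blueprint that advances missions when the first-person player character enters its overlap sphere.
; Once mission index 1 is complete, an overlap progresses missions 2 and 3; once both are complete, one progresses mission 4.
; DoOnce gates make each update fire a single time.
; UpdateMissionBehavior is empty, with disconnected logic for copying mission started and finished states to AI Blackboard keys built from mission names.
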(event OnComponentBeginOverlap(Sphere)
  (params (OverlappedComponent :type Primitive%20Component%20Object%20Reference) (OtherActor :type Actor%20Object%20Reference) (OtherComp :type Primitive%20Component%20Object%20Reference) (OtherBodyIndex :type Integer) (bFromSweep :type Boolean) (SweepResult :type Hit%20Result%20Structure%20%28by%20ref%29))
  (bind _missions (Variables|Default|GetMissions))
  (Utilities|Casting|CastToFirstPersonCharacter OtherActor)
  (Utilities|FlowControl|Sequence
    (:then_0
      (if (Variables|/Game/FirstPersonBP/Blueprints/MissionSystem/MissionManager.MissionManager_C|GetbMissionCompleted (Utilities|Array|Get(acopy) (Variables|Default|GetMissions) 1))
        (Utilities|FlowControl|DoOnce false
          (:Completed
            (Default|UpdateProgress (Utilities|Array|Get(acopy) _missions 2) 1)
            (Default|UpdateProgress (Utilities|Array|Get(acopy) _missions 3) 1)))))
    (:then_1
      (if (and (Variables|/Game/FirstPersonBP/Blueprints/MissionSystem/MissionManager.MissionManager_C|GetbMissionCompleted (Utilities|Array|Get(acopy) (Variables|Default|GetMissions) 2)) (Variables|/Game/FirstPersonBP/Blueprints/MissionSystem/MissionManager.MissionManager_C|GetbMissionCompleted (Utilities|Array|Get(acopy) (Variables|Default|GetMissions) 3)))
        (Utilities|FlowControl|DoOnce false
          (:Completed
            (Default|UpdateProgress (Utilities|Array|Get(acopy) (Variables|Default|GetMissions) 4) 1)))))))

(event EventBeginPlay)

(fn ConstructionScript)

(fn UpdateMissionBehavior)