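; AI controller for the Lilith character that runs her behavior tree and reports when she sees the player.
; On possess it stores the Lilith pawn and starts Lilith_BT.
; AI Perception updates that concern the FirstPersonCharacter copy the sensed state into Lilith's SeePlayer flag and the SeePlayer blackboard key, so both follow gaining and losing the player.
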(event OnTargetPerceptionUpdated(AIPerception)
  (params (Actor :type Actor%20Object%20Reference) (Stimulus :type AI%20Stimulus%20Structure))
  (bind _asfirst_person_character (Utilities|Casting|CastToFirstPersonCharacter Actor))
  (Variables|Default|SetPlayer _asfirst_person_character)
  (bind _output_get (Variables|/Game/Lilith_Character/Lilith_BPs/Lilith_CharacterBP.Lilith_CharacterBP_C|SetSeePlayer (Variables|Default|GetLilith) (.bSuccessfullySensed (Utilities|Struct|BreakAIStimulus Stimulus))))
  (AI|Components|Blackboard|SetValueasBool (AI|GetBlackboard 0) (Utilities|Name|MakeLiteralName "SeePlayer") _output_get))

(event EventBeginPlay)

(event EventTick
  (params (DeltaSeconds :type Float%20%28single-precision%29)))

(event EventOnPossess
  (params (PossessedPawn :type Pawn%20Object%20Reference))
  (bind _aslilith_character_bp (Utilities|Casting|CastToLilith_CharacterBP PossessedPawn))
  (Variables|Default|SetLilith _aslilith_character_bp)
  (AI|RunBehaviorTree "/Game/Lilith_Character/Lilith_BPs/Lilith_BT.Lilith_BT"))

(fn ConstructionScript)